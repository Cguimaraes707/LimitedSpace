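; Lava hazard actor that rises by stretching a Cube vertically and kills the player on contact.
; After a short start delay, a looping Timeline adds its Growth value to the Cube's Z scale whenever Blocked is false.
; Activate alternates between unblocking with rising-lava music and blocking again, while Deactivate is empty.
; Tick polls for player overlap, calling KillMessage on Controlplayer1 and playing a death sound every overlapping frame.
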(event EventBeginPlay
  (bind _cube (Variables|Default|GetCube))
  (bind _returnvalue (Transformation|GetWorldScale _cube))
  (Utilities|FlowControl|Delay 5.0)
  (bind _growth (Timeline|Timeline Play)
    (:Update
      (if (not (Variables|Default|GetBlocked))
        (Transformation|SetWorldScale3D _cube (Math|Vector|MakeVector (.x _returnvalue) (.y _returnvalue) (+ (.z _returnvalue) _growth)))))
    (:Finished
      (Timeline|Timeline PlayFromStart))))

(event Collision|EventActorBeginOverlap
  (params (OtherActor :type Actor%20Object%20Reference)))

(event EventTick
  (params (DeltaSeconds :type Float%20%28single-precision%29))
  (if (Collision|IsOverlappingActor (Variables|Default|GetCube) (Game|GetPlayerCharacter 0) :!class /Script/Engine.PrimitiveComponent)
    (bind _ascontrolplayer_1 (Utilities|Casting|CastToControlplayer1 (Game|GetPlayerController 0)))
    (Class|Kill|Kill(Message) _ascontrolplayer_1)
    (Audio|PlaySound2D "/Game/Audio/Death1.Death1" 1.0 1.0 0.0 0 0)))

(event EventActivate
  (Utilities|FlowControl|FlipFlop
    (:A
      (Variables|Default|SetBlocked false)
      (Audio|PlaySound2D "/Game/Audio/Lava_Rising_Music.Lava_Rising_Music" 1.0 1.0 0.0 0 0))
    (:B
      (Variables|Default|SetBlocked true))))

(event EventDeactivate)

(fn ConstructionScript)