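; Door Blueprint that the player opens with the E key when carrying the matching key number.
; Box overlap with the first-person character enables or disables input, so E only works near the door.
; On press, it checks the Controlplayer1 controller's Keys for KeyNum and plays a Timeline that yaws StaticMesh1.
; Without the key, a widget component shows for a short delay, then hides again.
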(event OnComponentBeginOverlap(Box)
  (params (OverlappedComponent :type Primitive%20Component%20Object%20Reference) (OtherActor :type Actor%20Object%20Reference) (OtherComp :type Primitive%20Component%20Object%20Reference) (OtherBodyIndex :type Integer) (bFromSweep :type Boolean) (SweepResult :type Hit%20Result%20Structure%20%28by%20ref%29))
  (Utilities|Casting|CastToBP_FirstPersonCharacter OtherActor)
  (Input|EnableInput (Game|GetPlayerController 0)))

(event OnComponentEndOverlap(Box)
  (params (OverlappedComponent :type Primitive%20Component%20Object%20Reference) (OtherActor :type Actor%20Object%20Reference) (OtherComp :type Primitive%20Component%20Object%20Reference) (OtherBodyIndex :type Integer))
  (Utilities|Casting|CastToBP_FirstPersonCharacter OtherActor)
  (Input|DisableInput (Game|GetPlayerController 0)))

(event Input|KeyboardEvents|E
  (params (Key :type Key%20Structure :default "None"))
  (bind _widget (Variables|Default|GetWidget))
  (:Pressed
    (bind _ascontrolplayer_1 (Utilities|Casting|CastToControlplayer1 (Game|GetPlayerController 0)))
    (if (Utilities|Array|ContainsItem (Variables|/Game/FirstPerson/Blueprints/Controlplayer1.Controlplayer1_C|GetKeys _ascontrolplayer_1) (Variables|Default|GetKeyNum))
      (bind _newtrack_0 (Timeline|Timeline Play)
        (:Update
          (Transformation|SetRelativeRotation (Variables|Default|GetStaticMesh1) (Math|Rotator|MakeRotator 0.0 0.0 (.y _newtrack_0)) false false)))
      (else
        (Development|SetHiddeninGame _widget false false)
        (Utilities|FlowControl|Delay 2.0)
        (Development|SetHiddeninGame _widget true false)))))

(fn ConstructionScript)