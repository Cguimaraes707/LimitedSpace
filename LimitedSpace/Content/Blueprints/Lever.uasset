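; Lever is an interactable lever that the first-person character operates with the E key to send activation messages to linked actors.
; Box overlap enables or disables the lever's input for the player.
; A FlipFlop alternates each press, calling ActivateMessage on every entry in the Activatee array both times.
; The Rotate timeline plays or reverses in step, pitching the Handle.
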(event OnComponentBeginOverlap(Box)
  (params (OverlappedComponent :type Primitive%20Component%20Object%20Reference) (OtherActor :type Actor%20Object%20Reference) (OtherComp :type Primitive%20Component%20Object%20Reference) (OtherBodyIndex :type Integer) (bFromSweep :type Boolean) (SweepResult :type Hit%20Result%20Structure%20%28by%20ref%29))
  (Utilities|Casting|CastToBP_FirstPersonCharacter OtherActor)
  (Input|EnableInput (Game|GetPlayerController 0)))

(event OnComponentEndOverlap(Box)
  (params (OverlappedComponent :type Primitive%20Component%20Object%20Reference) (OtherActor :type Actor%20Object%20Reference) (OtherComp :type Primitive%20Component%20Object%20Reference) (OtherBodyIndex :type Integer))
  (Utilities|Casting|CastToBP_FirstPersonCharacter OtherActor)
  (Input|DisableInput (Game|GetPlayerController 0)))

(event Input|KeyboardEvents|E
  (params (Key :type Key%20Structure :default "None"))
  (bind _activatee (Variables|Default|GetActivatee))
  (:Pressed
    (Utilities|FlowControl|FlipFlop
      (:A
        (for _array_element _activatee
          (Class|Activate|Activate(Message) _array_element))
        (bind _newtrack_0 (Timeline|Rotate Play)
          (:Update
            (Transformation|SetRelativeRotation (Variables|Default|GetHandle) (Math|Rotator|MakeRotator 0.0 (.y _newtrack_0) 0.0) false false))))
      (:B
        (for _array_element_2 _activatee
          (Class|Activate|Activate(Message) _array_element_2))
        (Timeline|Rotate Reverse)))))

(fn ConstructionScript)